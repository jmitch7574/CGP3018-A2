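; BP_Lightbulb is a toggleable bulb that recolours its emissive mesh and point light between enabled and disabled colours.
; UpdateLight applies the state instantly from construction, BeginPlay and Toggle, also setting the isOn parameter on linked powerline materials.
; The OnToggle and OnTurnOff events instead blend colours through the LightChange timeline, played forward or reversed, without updating powerlines.
; BeginPlay creates dynamic material instances for bulb and powerlines.
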(event Custom|OnLightChange
  (if (Variables|Default|GetIsOn)
    (bind _lighttrack (Timeline|LightChange PlayFromStart)
      (:Update
        (Rendering|Material|SetColorParameterValueonMaterials (Variables|Default|GetLightMesh) "LightColour" (Math|Color|Lerp(LinearColor) (Math|Conversions|ToLinearColor(Color) (Variables|Default|GetColorEnabled)) (Math|Conversions|ToLinearColor(Color) (Variables|Default|GetColorDisabled)) _lighttrack))
        (Rendering|Components|Light|SetLightColor (Variables|Default|GetPointLight) (Math|Color|Lerp(LinearColor) (Math|Conversions|ToLinearColor(Color) (Variables|Default|GetColorEnabled)) (Math|Conversions|ToLinearColor(Color) (Variables|Default|GetColorDisabled)) _lighttrack) true)))
    (else
      (Timeline|LightChange ReverseFromEnd))))

(event Custom|OnTurnOff
  (Variables|Default|SetIsOn false)
  (CallFunction|OnLightChange))

(event Custom|OnToggle
  (Variables|Default|SetIsOn (not (Variables|Default|GetIsOn)))
  (CallFunction|OnLightChange))

(event EventBeginPlay
  (bind _returnvalue (Rendering|Material|CreateDynamicMaterialInstance (Variables|Default|GetLightMesh) 0 "/Game/MyContent/Materials/M_EmissiveBulb.M_EmissiveBulb" "None" :!class /Script/Engine.PrimitiveComponent))
  (Variables|Default|SetThisBulbMaterialInstance _returnvalue)
  (CallFunction|UpdateLight)
  (for _array_element (Variables|Default|GetPowerlines)
    (Rendering|Material|CreateDynamicMaterialInstance (Variables|/Script/Engine.StaticMeshActor|GetStaticMeshComponent _array_element) 0 "/Game/MyContent/Materials/M_Powerline.M_Powerline" "None" :!class /Script/Engine.PrimitiveComponent)))

(fn ConstructionScript
  (CallFunction|UpdateLight))

(fn Toggle
  (Variables|Default|SetIsOn (not (Variables|Default|GetIsOn)))
  (CallFunction|UpdateLight))

(fn UpdateLight
  (bind _colorenabled (Variables|Default|GetColorEnabled))
  (bind _colordisabled (Variables|Default|GetColorDisabled))
  (bind _ison (Variables|Default|GetIsOn))
  (bind _returnvalue (select _ison _colorenabled _colordisabled))
  (Rendering|Material|SetColorParameterValueonMaterials (Variables|Default|GetLightMesh) "LightColour" (Math|Conversions|ToLinearColor(Color) _returnvalue))
  (Rendering|Components|Light|SetLightColor (Variables|Default|GetPointLight) (Math|Conversions|ToLinearColor(Color) _returnvalue) true)
  (CallFunction|UpdatePowerlines))

(fn UpdatePowerlines
  (for _array_element (Variables|Default|GetPowerlines)
    (Rendering|Material|SetScalarParameterValueonMaterials (Variables|/Script/Engine.StaticMeshActor|GetStaticMeshComponent _array_element) "isOn" (Math|Conversions|ToFloat(Boolean) (Variables|Default|GetIsOn)))))