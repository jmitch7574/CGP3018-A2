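; Security guard AI character that roams the level, chases pawns it sees and sends the player back to a respawn point on contact.
; It walks to random navigable points with a pause between moves.
; PawnSensing raises its speed and starts a chase, with a retriggerable delay returning it to slower roaming once sightings stop.
; Capsule overlap with the third-person character teleports them and turns off the referenced lights.
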(event OnSeePawn(PawnSensing)
  (params (Pawn :type Pawn%20Object%20Reference))
  (Variables|/Script/Engine.CharacterMovementComponent|SetMaxWalkSpeed (Variables|Character|GetCharacterMovement) 4e+02)
  (AI|AIMoveTo self "0, 0, 0" Pawn 3.0 false
    (:then
      (Utilities|FlowControl|RetriggerableDelay 2.0)
      (CallFunction|MovetoRandomLocation))))

(event OnComponentBeginOverlap(Capsule)
  (params (OverlappedComponent :type Primitive%20Component%20Object%20Reference) (OtherActor :type Actor%20Object%20Reference) (OtherComp :type Primitive%20Component%20Object%20Reference) (OtherBodyIndex :type Integer) (bFromSweep :type Boolean) (SweepResult :type Hit%20Result%20Structure%20%28by%20ref%29))
  (bind _asbp_third_person_character (Utilities|Casting|CastToBP_ThirdPersonCharacter OtherActor))
  (Transformation|SetActorLocation _asbp_third_person_character (Transformation|GetActorLocation (Variables|Default|GetPlayerRespawnPoint)) false true)
  (for _array_element (Variables|Default|GetLights)
    (Default|OnTurnOff _array_element)))

(event Custom|MoveToRandomLocation
  (bind _randomlocation (Class|NavigationSystemV1|GetRandomLocationinNavigableRadius (Transformation|GetActorLocation) 1.5e+03 0 0))
  (Variables|/Script/Engine.CharacterMovementComponent|SetMaxWalkSpeed (Variables|Character|GetCharacterMovement) 2e+02)
  (AI|AIMoveTo self _randomlocation 0 5.0 false
    (:OnSuccess
      (Utilities|FlowControl|Delay 3.0)
      (CallFunction|MovetoRandomLocation))))

(event EventBeginPlay
  (CallFunction|MovetoRandomLocation))

(fn ConstructionScript)