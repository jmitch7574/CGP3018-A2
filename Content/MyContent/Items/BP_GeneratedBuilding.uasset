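; BP_GeneratedBuilding is a procedural building that generates a box body with a flat, lipped roof from its Bounds.
; On mesh rebuild it appends boxes with collision for the body and a thin roof slab, then calls CreateLip once per edge direction for the rim.
; Remapping material IDs after each of the first two boxes gives brick walls and a blackstone roof, leaving the lips on the rooflip material.
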(event Events|EventOnRebuildGeneratedMesh
  (params (TargetMesh :type Dynamic%20Mesh%20Object%20Reference))
  (bind _bounds (Variables|Default|GetBounds))
  (bind _bounds_2 (Variables|Default|GetBounds))
  (bind _bounds_3 (Variables|Default|GetBounds))
  (Class|DynamicMeshComponent|ConfigureMaterialSet (Variables|DynamicMeshActor|GetDynamicMeshComponent) (Utilities|Array|MakeArray "/Game/MyContent/Materials/M_Rooflip.M_Rooflip" "/Game/MyContent/Materials/MI_Stone_Blackstone.MI_Stone_Blackstone" "/Game/MyContent/Materials/MI_Brick.MI_Brick") false)
  (bind _output_get (Variables|Default|SetLipWidth 4e+01))
  (Variables|Default|SetHalfLipWidth (/ _output_get 2.0))
  (bind _returnvalue (Class|GeometryScriptLibraryMeshPrimitiveFunctions|AppendBoxwithCollision :TargetMesh TargetMesh :Transform (Math|Transform|MakeTransform (Math|Vector|MakeVector (/ (.x _bounds_3) 2.0) (/ (.y _bounds_3) 2.0) 0.0)) :DimensionX (.x _bounds_2) :DimensionY (.y _bounds_2) :DimensionZ (.z _bounds_2) :Debug 0))
  (bind _returnvalue_2 (GeometryScript|Materials|RemapMaterialIDs _returnvalue 0 2 0))
  (bind _returnvalue_3 (Class|GeometryScriptLibraryMeshPrimitiveFunctions|AppendBoxwithCollision :TargetMesh _returnvalue_2 :Transform (Math|Transform|MakeTransform (Math|Vector|MakeVector (/ (.x _bounds) 2.0) (/ (.y _bounds) 2.0) (.z _bounds))) :DimensionX (.x _bounds) :DimensionY (.y _bounds) :DimensionZ 5.0 :Debug 0))
  (bind _returnvalue_4 (GeometryScript|Materials|RemapMaterialIDs _returnvalue_3 0 1 0))
  (bind _targetmeshout (CallFunction|CreateLip _returnvalue_4 "1.000000,0.000000,0.000000"))
  (bind _targetmeshout_2 (CallFunction|CreateLip _targetmeshout "-1.000000,0.000000,0.000000"))
  (bind _targetmeshout_3 (CallFunction|CreateLip _targetmeshout_2 "0.000000,1.000000,0.000000"))
  (CallFunction|CreateLip _targetmeshout_3 "0.000000,-1.000000,0.000000"))

(fn ConstructionScript)

(fn CreateLip
  (params (TargetMesh :type Dynamic%20Mesh%20Object%20Reference) (Rotation :type Vector))
  (bind _bounds (Variables|Default|GetBounds))
  (bind _bounds_2 (Variables|Default|GetBounds))
  (bind _bounds_3 (Variables|Default|GetBounds))
  (bind _halflipwidth (Variables|Default|GetHalfLipWidth))
  (LocalVariables|SetEdge Rotation)
  (bind _returnvalue (Class|GeometryScriptLibraryMeshPrimitiveFunctions|AppendBoxwithCollision :TargetMesh TargetMesh :Transform (Math|Transform|MakeTransform (Math|Vector|MakeVector (+ (* (- (.x _bounds_2) _halflipwidth) (/ (.x (LocalVariables|GetEdge)) 2.0)) (/ (.x _bounds_3) 2.0)) (+ (* (- (.y _bounds_2) _halflipwidth) (/ (.y (LocalVariables|GetEdge)) 2.0)) (/ (.y _bounds_3) 2.0)) (.z (Variables|Default|GetBounds))) (Math|Rotator|MakeRotator 0.0 0.0 (* (.x (LocalVariables|GetEdge)) 9e+01))) :DimensionX (select (== (.y (LocalVariables|GetEdge)) 0.0) (.y _bounds) (.x _bounds)) :DimensionY (Variables|Default|GetLipWidth) :DimensionZ 25.0 :Debug 0))
  (return _returnvalue))