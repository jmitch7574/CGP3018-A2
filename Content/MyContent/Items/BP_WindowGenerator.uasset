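; BP_WindowGenerator is a construction-time generator that fills a rectangular area with a grid of window child actors.
; The construction script destroys the components stored in SpawnedWindows, then derives column and row counts from Bounds Y and Z divided by window width and height.
; Nested loops add a Child Actor Component at each half-cell-offset position on the local YZ plane and record it in SpawnedWindows.
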(event EventBeginPlay)

(event Collision|EventActorBeginOverlap
  (params (OtherActor :type Actor%20Object%20Reference)))

(event EventTick
  (params (DeltaSeconds :type Float%20%28single-precision%29)))

(fn ConstructionScript
  (for _array_element (Variables|Default|GetSpawnedWindows)
    (Components|DestroyComponent _array_element))
  (Variables|Default|SetColumns (Math|Float|Truncate (/ (.y (Variables|Default|GetBounds)) (Variables|Default|GetWindowWidth))))
  (Variables|Default|SetRows (Math|Float|Truncate (/ (.z (Variables|Default|GetBounds)) (Variables|Default|GetWindowHeight))))
  (for _index (range 0 (Variables|Default|GetColumns))
    (for _index_2 (range 0 (Variables|Default|GetRows))
      (bind _returnvalue (AddComponent|AddChildActorComponent false (Math|Transform|MakeTransform (Math|Vector|MakeVector 0.0 (+ (* _index (Variables|Default|GetWindowWidth)) (/ (Variables|Default|GetWindowWidth) 2.0)) (+ (* _index_2 (Variables|Default|GetWindowHeight)) (/ (Variables|Default|GetWindowHeight) 2.0))))))
      (Utilities|Array|Add (Variables|Default|GetSpawnedWindows) _returnvalue))))