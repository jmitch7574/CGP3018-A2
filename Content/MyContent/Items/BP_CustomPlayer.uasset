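; BP_CustomPlayer is the player character Blueprint, adding a lever-pull interaction.
; TriggerLever snaps the character to a given stand position and facing, then sets a forward or reversed pull flag on its ABP_Unarmed anim instance.
; It disables player 0 input and starts a fixed timer, after which reEnableInput clears both flags and restores control.
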(event EventBeginPlay)

(event Collision|EventActorBeginOverlap
  (params (OtherActor :type Actor%20Object%20Reference)))

(event EventTick
  (params (DeltaSeconds :type Float%20%28single-precision%29)))

(fn ConstructionScript
  (|CallParentFunction))

(fn TriggerLever
  (params (IsReversed :type Boolean) (standPosition :type Vector) (standDirection :type Rotator))
  (Transformation|SetActorLocation standPosition false false)
  (Transformation|SetActorRotation standDirection)
  (bind _asabp_unarmed (Utilities|Casting|CastToABP_Unarmed (Components|SkeletalMesh|GetAnimInstance (Variables|Character|GetMesh))))
  (if IsReversed
    (Variables|/Game/Characters/Mannequins/Anims/Unarmed/ABP_Unarmed.ABP_Unarmed_C|SetShouldLeverPull_Reversed _asabp_unarmed true)
    (else
      (Variables|/Game/Characters/Mannequins/Anims/Unarmed/ABP_Unarmed.ABP_Unarmed_C|SetShouldLeverPull _asabp_unarmed true)))
  (Input|DisableInput (Game|GetPlayerController 0))
  (Utilities|Time|SetTimerbyFunctionName 0 "reEnableInput" 1.5))

(fn ReEnableInput
  (bind _asabp_unarmed (Utilities|Casting|CastToABP_Unarmed (Components|SkeletalMesh|GetAnimInstance (Variables|Character|GetMesh))))
  (Variables|/Game/Characters/Mannequins/Anims/Unarmed/ABP_Unarmed.ABP_Unarmed_C|SetShouldLeverPull _asabp_unarmed false)
  (Variables|/Game/Characters/Mannequins/Anims/Unarmed/ABP_Unarmed.ABP_Unarmed_C|SetShouldLeverPull_Reversed _asabp_unarmed false)
  (Input|EnableInput (Game|GetPlayerController 0)))